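; Radar actor Blueprint that places itself on a Cesium globe at a location fetched from a backend service.
; On BeginPlay it GETs the radar locate endpoint, moves its globe anchor to the returned longitude and latitude at a fixed height, and caches that transform for Reset to restore.
; Cursor hover begin and end events broadcast pointer or default cursor JSON messages to all clients through the level's SocketServer actor.
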(event `self.ReceiveBeginPlay`
  (`|ExecutionSequence`
    (:`then_0`
      (bind (_outheader _result_body) (`|HttpRequest` (`KismetStringLibrary.Concat_StrStr` (`self.baseUrl`) "/v1/smart3d/radar/locate") "Get")
        (:`On Success`
          (`|ExecutionSequence`
            (:`then_0`
              (bind _outvalue (`|GetJsonField` _result_body "lng")))
            (:`then_1`
              (bind _outvalue_2 (`|GetJsonField` _result_body "lat"))
              (`CesiumGlobeAnchorComponent.MoveToLongitudeLatitudeHeight` (`self.CesiumGlobeAnchor`) (`KismetMathLibrary.MakeVector` _outvalue _outvalue_2 1400.0))
              (set `self.radarTransform` (`self.GetTransform`)))))))
    (:`then_1`
      (bind _returnvalue (`GameplayStatics.GetActorOfClass` "/Game/blueprints/SocketServer.SocketServer_C"))
      (add `self.OnBeginCursorOver` (delegate `OnBeginCursorOver_Event`))
      (add `self.OnEndCursorOver` (delegate `OnEndCursorOver_Event`)))))

(event `OnBeginCursorOver_Event` :!signature `self.OnBeginCursorOver`
  (params (TouchedActor :type "Actor Object Reference"))
  (`DsWebSocketServer.SendToAllClients` (`/Game/blueprints/SocketServer.socketServer` (stale `self.ReceiveBeginPlay` _returnvalue)) "{\"type\":\"cursorPointer\"}"))

(event `OnEndCursorOver_Event` :!signature `self.OnEndCursorOver`
  (params (TouchedActor :type "Actor Object Reference"))
  (`DsWebSocketServer.SendToAllClients` (`/Game/blueprints/SocketServer.socketServer` (stale `self.ReceiveBeginPlay` _returnvalue)) "{\"type\":\"cursorDefault\"}"))

(fn `reset`
  (`self.K2_SetActorTransform` (`self.radarTransform`)))

(fn `UserConstructionScript`)