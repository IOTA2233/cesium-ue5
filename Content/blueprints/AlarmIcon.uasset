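; Clickable world alarm marker that stores alarm data and tints its icon by alarm level through a dynamic material.
; Cursor hover raises the material's light parameter to highlight the icon.
; Clicking flies the first DynamicPawn to the alarm's longitude, latitude and height via its FlyTo component.
; A changeLight event scales the icon by player distance, but its looping timer is disconnected and nothing here calls it.
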(event `self.ReceiveBeginPlay`
  ;[1 1 1] 等比缩放actor
)

(event `changeLight`
  ;[1 1 1] 等比缩放actor
  (`SceneComponent.SetWorldScale3D` (`self.icon`) (`KismetMathLibrary.Conv_DoubleToVector` (/ (`KismetMathLibrary.Vector_Distance` (`self.K2_GetActorLocation` (`GameplayStatics.GetPlayerPawn` 0)) (`SceneComponent.K2_GetComponentLocation` (`self.DefaultSceneRoot`))) 2300.0))))

(event `self.collision.OnBeginCursorOver`
  (params (TouchedComponent :type "PrimitiveComponent Object Reference"))
  ;[1 1 1] 鼠标高亮
  (`self.setHighLightEnabled` true))

(event `self.collision.OnClicked`
  (params (TouchedComponent :type "PrimitiveComponent Object Reference") (ButtonPressed :type "Key Structure"))
  (bind (_longitude _latitude _height) (break `/Game/AlarmData` (`self.IconValue`)))
  ;[1 1 1] 点击定位
  (bind _outactors (`GameplayStatics.GetAllActorsOfClass` "/CesiumForUnreal/DynamicPawn.DynamicPawn_C"))
  (`CesiumFlyToComponent.FlyToLocationLongitudeLatitudeHeight` (`/CesiumForUnreal/DynamicPawn.FlyTo` (`|GetArrayItem` _outactors)) (`KismetMathLibrary.MakeVector_NetQuantize` _longitude _latitude _height) 135.0 -40.0 false))

(event `self.collision.OnEndCursorOver`
  (params (TouchedComponent :type "PrimitiveComponent Object Reference"))
  ;[1 1 1] 鼠标高亮
  (`self.setHighLightEnabled` false)
  (`KismetSystemLibrary.PrintText` "离开悬停状态"))

(fn `changeMaterial`
  (params (AlarmData :type "/Game/AlarmData Structure"))
  (locals (color :type "Vector Structure"))
  (bind _dmi (`self.DMI`))
  (set `self.IconValue` AlarmData)
  (switch `string` (`KismetStringLibrary.Conv_IntToString` (`.level_10_5717388A4169F606F8C06BB80005DD47` (break `/Game/AlarmData` AlarmData)))
    (:`1`
      (`MaterialInstanceDynamic.SetVectorParameterValue` _dmi "color" (make `LinearColor` 1.0 0.0 0.0 1.0)))
    (:`2`
      (`MaterialInstanceDynamic.SetVectorParameterValue` _dmi "color" (make `LinearColor` 1.0 0.141263 0.0 1.0)))
    (:`3`
      (`MaterialInstanceDynamic.SetVectorParameterValue` _dmi "color" (make `LinearColor` 0.955974 0.708376 0.006995 1.0)))
    (:`4`
      (`MaterialInstanceDynamic.SetVectorParameterValue` _dmi "color" (make `LinearColor` 0.001821 0.291771 0.768151 1.0)))))

(fn `setHighLightEnabled`
  (params (isActive :type Boolean))
  (bind _dmi (`self.DMI`))
  (if isActive
    (`MaterialInstanceDynamic.SetScalarParameterValue` _dmi "light" 30.0)
    (else
      (`MaterialInstanceDynamic.SetScalarParameterValue` _dmi "light" 5.0))))

(fn `UserConstructionScript`
  (bind _returnvalue (`PrimitiveComponent.CreateDynamicMaterialInstance` (`self.icon`) 0 (`PrimitiveComponent.GetMaterial` (`self.icon`) 0) "None"))
  (bind _output_get (set `self.DMI` _returnvalue))
  (`PrimitiveComponent.SetMaterial` (`self.icon`) 0 _output_get))